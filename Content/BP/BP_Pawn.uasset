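; Player pawn for a cell-simulation board, providing an orthographic camera, mouse cell editing and the game UI.
; On BeginPlay it polls the game mode until the board exists, centers on its tilemap and creates W_Game, whose events start, stop and retime the simulation.
; Holding left or middle mouse runs a gated delay loop that traces under the cursor to add or remove cells.
; Right mouse enables panning; the Zoom axis adjusts ortho width.
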(event `self.ReceiveBeginPlay`
  (bind _returnvalue (`GameplayStatics.GetPlayerController` 0))
  (`WidgetBlueprintLibrary.SetInputMode_GameAndUIEx` _returnvalue null "DoNotLock" false)
  (set `PlayerController.bShowMouseCursor` true _returnvalue)
  (`KismetSystemLibrary.Delay` 0.2 :!label _label)
  (bind _asgmb_game (cast `/Game/Core/GMB_Game` (`GameplayStatics.GetGameMode`)))
  (bind _board (`GameOfLifeGM.Board` _asgmb_game)
    (:`then`
      (bind _asbp_board (cast `/Game/BP/BP_Board` _board) ; todo
        (:`then`
          (set `self.BP Board` _asbp_board))
        (:`CastFailed`
          _))
      (bind _origin (`KismetSystemLibrary.GetComponentBounds` (`Board.TileMap` _board)))
      (`self.K2_SetActorTransform` (`KismetMathLibrary.MakeTransform` (`KismetMathLibrary.MakeVector` (.x _origin) (+ (.y _origin) 300.0) (.z _origin)) (struct :`Yaw` -90.0)))
      (bind _returnvalue_2 (`|CreateWidget` "/Game/Widgets/W_Game.W_Game_C" (`GameplayStatics.GetPlayerController` 0)))
      (`UserWidget.AddToViewport` _returnvalue_2 0)
      (add `/Game/Widgets/W_Game.OnStart` _returnvalue_2 (delegate `OnStart_UI`))
      (add `/Game/Widgets/W_Game.OnRefreshChanged` _returnvalue_2 (delegate `OnRefreshChanged_UI`)))
    (:`else`
      (goto _label))))

(event `OnStart_UI`
  (params (Stop :type Boolean))
  (bind _bp_board (`self.BP Board`)
    (:`then`
      (if Stop
        (`/Game/BP/BP_Board.StopSimulation` _bp_board)
        (else
          (`/Game/BP/BP_Board.StartSimulation` _bp_board))))
    (:`else`)))

(event `OnRefreshChanged_UI`
  (params (NewRate :type "Float (double-precision)"))
  (bind _bp_board (`self.BP Board`)
    (:`then`
      (`/Game/BP/BP_Board.ChangeRate` _bp_board NewRate))
    (:`else`)))

(event `Key|LeftMouseButton`
  (params (Key :type "Key Structure"))
  (:`Pressed`
    (`|ExecutionSequence`
      (:`then_0`
        (goto _label_2 :!via `Open`))
      (:`then_1`
        (`/Engine/EditorBlueprintResources/StandardMacros.Gate` true :!label _label_2
          (:`Exit`
            (bind (_asbp_board _hitcomponent _success) (`self.TraceCell`))
            (if _success
              (`/Game/BP/BP_Board.AddCellFromMouse` _asbp_board _hitcomponent false))
            (`KismetSystemLibrary.Delay` 0.02)
            (goto _label_2))))))
  (:`Released`
    (goto _label_2 :!via `Close`)))

(event `Key|MiddleMouseButton`
  (params (Key :type "Key Structure"))
  (:`Pressed`
    (`|ExecutionSequence`
      (:`then_0`
        (goto _label_3 :!via `Open`))
      (:`then_1`
        (`/Engine/EditorBlueprintResources/StandardMacros.Gate` true :!label _label_3
          (:`Exit`
            (bind (_asbp_board _hitcomponent _success) (`self.TraceCell`))
            (if _success
              (`/Game/BP/BP_Board.AddCellFromMouse` _asbp_board _hitcomponent true))
            (`KismetSystemLibrary.Delay` 0.02)
            (goto _label_3))))))
  (:`Released`
    (goto _label_3 :!via `Close`)))

(event `InputAxis|Zoom`
  (params (AxisValue :type "Float (single-precision)"))
  (bind _camera (`self.Camera`))
  (`CameraComponent.SetOrthoWidth` _camera (+ (* -100 AxisValue) (`CameraComponent.OrthoWidth` _camera))))

(event `self.ReceiveTick`
  (params (DeltaSeconds :type "Float (single-precision)"))
  (bind (_returnvalue_x _returnvalue_y _returnvalue_z) (`KismetMathLibrary.BreakVector` (`self.K2_GetActorLocation`)))
  (`/Engine/EditorBlueprintResources/StandardMacros.Gate` true :!label _label_4
    (:`Exit`
      (`self.K2_SetActorLocation` (`KismetMathLibrary.MakeVector` (+ _returnvalue_x (* (`self.GetInputAxisKeyValue`) -5.0)) _returnvalue_y (+ _returnvalue_z (* (`self.GetInputAxisKeyValue`) -5.0)))))))

(event `Key|RightMouseButton`
  (params (Key :type "Key Structure"))
  (:`Pressed`
    (goto _label_4 :!via `Open`))
  (:`Released`
    (goto _label_4 :!via `Close`)))

(fn `TraceCell`
  (returns (`AsBP Board` :type "/Game/BP/BP_Board Object Reference") (HitComponent :type "PrimitiveComponent Object Reference") (Success :type Boolean))
  (bind (_worldlocation _worlddirection) (`PlayerController.DeprojectMousePositionToWorld` (`GameplayStatics.GetPlayerController` 0)))
  (bind (_outhit _returnvalue) (`KismetSystemLibrary.LineTraceSingle` _worldlocation (+ _worlddirection (* _worlddirection 10000000.0)) "TraceTypeQuery1"))
  (if _returnvalue
    (bind (_bblockinghit _binitialoverlap _time _distance _location _impactpoint _normal _impactnormal _physmat _hitactor _hitcomponent) (`GameplayStatics.BreakHitResult` _outhit))
    (bind _asbp_board (cast `/Game/BP/BP_Board` _hitactor)
      (:`then`
        (return _asbp_board _hitcomponent true))
      (:`CastFailed`
        _)))
  (return null null false))

(fn `UserConstructionScript`)