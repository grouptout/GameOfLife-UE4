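; Tile-map board for a cellular automaton, where cells are alive or dead and can be painted, erased, randomized, cleared or loaded from template maps.
; Edits keep the TileMap and AliveCells in sync, converting mouse locations to grid coordinates.
; A gated Delay loop calls UpdateCells, whose rules live outside this graph, at RefreshRate until stopped.
; UpdateTileStatetoMap redraws only changed tiles, and BeginPlay adds a box component sized to the map.
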(event `self.ReceiveBeginPlay`
  (bind (_origin _boxextent) (`KismetSystemLibrary.GetComponentBounds` (`self.TileMap`)))
  (bind _returnvalue (`AddComponent|NODE_AddBoxComponent-2` :`RelativeTransform` (`KismetMathLibrary.MakeTransform` _origin)))
  (`BoxComponent.SetBoxExtent` _returnvalue _boxextent false))

(event `AddCellFromMouse`
  (params (Loc :type "Vector Structure") (Remove :type Boolean))
  (bind _alivecells (`self.AliveCells`))
  (bind _returnvalue (`KismetMathLibrary.FTrunc` (/ (+ (.x Loc) 2.5) 5.0)))
  (bind _returnvalue_2 (`KismetMathLibrary.FTrunc` (/ (- (.z Loc) 2.5) -5.0)))
  (bind _intpoint (make `IntPoint` _returnvalue _returnvalue_2))
  (bind (_x _y) (break `IntPoint` _intpoint))
  (bind (_mapwidth _mapheight) (`PaperTileMapComponent.GetMapSize` (`self.TileMap`)))
  (if (and (>= _mapwidth _returnvalue) (>= _mapheight _returnvalue_2))
    (if Remove
      (if (`BlueprintSetLibrary.Set_Contains` _alivecells _intpoint)
        (`PaperTileMapComponent.SetTile` (`self.TileMap`) _x _y 0 (`TileMapBlueprintLibrary.MakeTile` 0))
        (`BlueprintSetLibrary.Set_Remove` _alivecells _intpoint))
      (else
        (`self.AddInitialTile` _x _y)))))

(event `ChangeRate`
  (params (`Refresh Rate` :type "Float (double-precision)"))
  (set `self.RefreshRate` `Refresh Rate`))

(event `StartSimulation`
  (`|ExecutionSequence`
    (:`then_0`
      (goto _label :!via `Open`))
    (:`then_1`
      (`/Engine/EditorBlueprintResources/StandardMacros.Gate` true :!label _label
        (:`Exit`
          (`self.UpdateCells`)
          (`KismetSystemLibrary.Delay` (`self.RefreshRate`))
          (goto _label))))))

(event `StopSimulation`
  (goto _label :!via `Close`))

(event `AddInitialTile`
  (params (X :type Integer) (Y :type Integer))
  (bind _alivecells (`self.AliveCells`))
  (if (not (`BlueprintSetLibrary.Set_Contains` _alivecells (make `IntPoint` X Y)))
    (`PaperTileMapComponent.SetTile` (`self.TileMap`) X Y 0 (`TileMapBlueprintLibrary.MakeTile` 0 "/Game/Tiles/TS_Game.TS_Game"))
    (`BlueprintSetLibrary.Set_Add` _alivecells (make `IntPoint` X Y))))

(event `self.UpdateTileStateToMap`
  (params (Coord :type "IntPoint Structure (by ref)") (Alive :type Boolean))
  (bind _tilemap (`self.TileMap`))
  (if (!= Alive (`KismetSystemLibrary.IsValid` (`.TileSet` (`TileMapBlueprintLibrary.BreakTile` (`PaperTileMapComponent.GetTile` _tilemap Coord_X Coord_Y 0)))))
    (`PaperTileMapComponent.SetTile` _tilemap Coord_X Coord_Y 0 (`TileMapBlueprintLibrary.MakeTile` 0 (select `bool` Alive :`true` "/Game/Tiles/TS_Game.TS_Game" :!type "PaperTileSet Object Reference")))))

(event `AddTemplate`
  (params (NewTemplae :type "PaperTileMap Object Reference"))
  (bind _returnvalue (`|AddComponentByClass` "/Script/Paper2D.PaperTileMapComponent" false (`KismetMathLibrary.MakeTransform` (0.0 0.0 0.0))))
  (bind _returnvalue_2 (`PaperTileMapComponent.SetTileMap` _returnvalue NewTemplae))
  (if _returnvalue_2
    (bind (_mapwidth _mapheight) (`PaperTileMapComponent.GetMapSize` _returnvalue))
    (for _index (range _mapwidth)
      (for _index_2 (range _mapheight)
        (`/Engine/EditorBlueprintResources/StandardMacros.IsValid` (`.TileSet` (`TileMapBlueprintLibrary.BreakTile` (`PaperTileMapComponent.GetTile` _returnvalue _index _index_2 0)))
          (:`Is Valid`
            (`self.AddInitialTile` _index _index_2))))))
  (`ActorComponent.K2_DestroyComponent` _returnvalue))

(event `ClearAll`
  (bind _tilemap (`self.TileMap`))
  (bind (_mapwidth _mapheight) (`PaperTileMapComponent.GetMapSize` _tilemap))
  (for _index (range _mapwidth)
    (for _index_2 (range _mapheight)
      (`/Engine/EditorBlueprintResources/StandardMacros.IsValid` (`.TileSet` (`TileMapBlueprintLibrary.BreakTile` (`PaperTileMapComponent.GetTile` _tilemap _index _index_2 0)))
        (:`Is Valid`
          (`PaperTileMapComponent.SetTile` (`self.TileMap`) _index _index_2 0 (`TileMapBlueprintLibrary.MakeTile` 0)))
        (:`Is Not Valid`
          _))
      (`BlueprintSetLibrary.Set_Remove` (`self.AliveCells`) (make `IntPoint` _index _index_2)))))

(event `GenerateRandom`
  (`self.ClearAll`)
  (bind (_mapwidth _mapheight) (`PaperTileMapComponent.GetMapSize` (`self.TileMap`)))
  (for _index (range _mapwidth)
    (for _index_2 (range _mapheight)
      (if (`KismetMathLibrary.RandomBool`)
        (`self.AddInitialTile` _index _index_2)))))

(fn `GetNearestTile`
  (params (Loc :type "Vector Structure"))
  (returns (CellCoords :type "IntPoint Structure"))
  (locals (Cell :type "IntPoint Structure") (Dist :type "Float (double-precision)" :default 10000000000.0) (L_TempDist :type "Float (double-precision)" :default 0.0))
  (bind _tilemap (`self.TileMap`))
  (bind (_mapwidth _mapheight) (`PaperTileMapComponent.GetMapSize` _tilemap))
  (for _index (range _mapwidth)
    (for _index_2 (range _mapheight)
      (bind _output_get (set `local.L_TempDist` (`KismetMathLibrary.Vector_Distance` Loc (`PaperTileMapComponent.GetTileCenterPosition` _tilemap _index _index_2 0 true))))
      (if (< _output_get (`local.Dist`))
        (set `local.Cell` (make `IntPoint` _index _index_2))
        (set `local.Dist` _output_get))))
  (return (`local.Cell`)))

(fn `UserConstructionScript`)